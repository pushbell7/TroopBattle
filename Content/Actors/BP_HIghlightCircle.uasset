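; BP_HighlightCircle is a decal actor that marks the spot under the cursor while a player selection is pending.
; It starts hidden and, each tick, shows its decal only while player 0's PlayerSelectionManagingSubsystem reports an active callback.
; While visible, it moves to the hit location of a complex Visibility trace under that player's mouse cursor.
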(event EventBeginPlay
  (Rendering|SetVisibility (Variables|Decal|GetDecal) false false))

(event EventTick
  (params (DeltaSeconds :type Float%20%28single-precision%29))
  (bind _returnvalue (Class|GameplayStatics|GetPlayerControllerfromID))
  (bind _returnvalue_2 (Subsystems|GetPlayerSelectionManagingSubsystem _returnvalue))
  (bind _returnvalue_3 (Class|PlayerSelectionManagingSubsystem|HasCallback _returnvalue_2))
  (Rendering|SetVisibility (Variables|Decal|GetDecal) _returnvalue_3 false)
  (if _returnvalue_3
    (Transformation|SetActorLocation (.Location (Collision|BreakHitResult (.HitResult (Game|Player|GetHitResultUnderCursorbyChannel _returnvalue "TraceTypeQuery1" true)))) false false)))

(fn ConstructionScript)